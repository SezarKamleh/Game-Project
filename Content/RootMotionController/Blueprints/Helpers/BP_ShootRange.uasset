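; BP_ShootRange is a shooting range target that falls when hit by a BP_MasterProjectile and raises itself again after a delay.
; A component hit plays the Drop timeline to roll the mesh down, then reverses it and clears the hit flags.
; Overlap zones for 100, 80 and 50 points each set a flag through a DoOnce.
; HitChecker picks the highest flagged zone, whose score is printed to screen.
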(event `self.StaticMeshComponent0.OnComponentHit`
  (params (HitComponent :type "PrimitiveComponent Object Reference") (OtherActor :type "Actor Object Reference") (OtherComp :type "PrimitiveComponent Object Reference") (NormalImpulse :type "Vector Structure") (Hit :type "HitResult Structure (by ref)"))
  (cast `/Game/RootMotionController/Blueprints/Weapon/Projectile/BP_MasterProjectile` OtherActor)
  (bind (_direction _newtrack_0) (`Timeline|Drop` :!label _label)
    (:`Update`
      (`SceneComponent.K2_SetRelativeRotation` (`self.StaticMeshComponent0`) (`KismetMathLibrary.MakeRotator` _newtrack_0) false false)
      (if (not (`self.DoOnce?`))
        (if (`KismetMathLibrary.NearlyEqual_FloatFloat` _newtrack_0 -90.0 0.1)
          (`/Engine/EditorBlueprintResources/StandardMacros.DoOnce` false :!label _label_2
            (:`Completed`
              (`KismetSystemLibrary.Delay` (`self.Delay`))
              (`self.Reset And Retrigger`)
              (set `self.100Hit` false)
              (set `self.80Hit` false)
              (set `self.50Hit` false)
              (`self.Reset Hit Result`)))
          (else
            (goto _label_2 :!via `Reset`)))))))

(event `Reset And Retrigger`
  (goto _label :!via `Reverse`))

(event `self.100.OnComponentBeginOverlap`
  (params (OverlappedComponent :type "PrimitiveComponent Object Reference") (OtherActor :type "Actor Object Reference") (OtherComp :type "PrimitiveComponent Object Reference") (OtherBodyIndex :type Integer) (bFromSweep :type Boolean) (SweepResult :type "HitResult Structure (by ref)"))
  (cast `/Game/RootMotionController/Blueprints/Weapon/Projectile/BP_MasterProjectile` OtherActor)
  (`/Engine/EditorBlueprintResources/StandardMacros.DoOnce` false :!label _label_3
    (:`Completed`
      (set `self.100Hit` true)
      (`self.HitChecker`
        (:`100Hit`
          (`KismetSystemLibrary.PrintString` "100"))))))

(event `Reset Hit Result`
  (`|ExecutionSequence`
    (:`then_0`
      (goto _label_3 :!via `Reset`))
    (:`then_1`
      (goto _label_4 :!via `Reset`))
    (:`then_2`
      (goto _label_5 :!via `Reset`))))

(event `self.80.OnComponentBeginOverlap`
  (params (OverlappedComponent :type "PrimitiveComponent Object Reference") (OtherActor :type "Actor Object Reference") (OtherComp :type "PrimitiveComponent Object Reference") (OtherBodyIndex :type Integer) (bFromSweep :type Boolean) (SweepResult :type "HitResult Structure (by ref)"))
  (cast `/Game/RootMotionController/Blueprints/Weapon/Projectile/BP_MasterProjectile` OtherActor)
  (`/Engine/EditorBlueprintResources/StandardMacros.DoOnce` false :!label _label_4
    (:`Completed`
      (set `self.80Hit` true)
      (`self.HitChecker`
        (:`80Hit`
          (`KismetSystemLibrary.PrintString` "80"))))))

(event `self.50.OnComponentBeginOverlap`
  (params (OverlappedComponent :type "PrimitiveComponent Object Reference") (OtherActor :type "Actor Object Reference") (OtherComp :type "PrimitiveComponent Object Reference") (OtherBodyIndex :type Integer) (bFromSweep :type Boolean) (SweepResult :type "HitResult Structure (by ref)"))
  (cast `/Game/RootMotionController/Blueprints/Weapon/Projectile/BP_MasterProjectile` OtherActor)
  (`/Engine/EditorBlueprintResources/StandardMacros.DoOnce` false :!label _label_5
    (:`Completed`
      (set `self.50Hit` true)
      (`self.HitChecker`
        (:`50Hit`
          (`KismetSystemLibrary.PrintString` "50"))))))

(fn `UserConstructionScript`)