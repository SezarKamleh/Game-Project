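; BP_NotificationTrigger is a one-shot trigger volume that shows an on-screen notification when a BP_MasterCharacter enters it.
; On overlap it passes its configured content to the character's RootMotionController as either a small or big notification, chosen by SmallNotification, then destroys itself.
; The construction script sizes the box, raises it so its base sits at the billboard's height, and copies Text to a TextRender label.
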(event `self.Box.OnComponentBeginOverlap`
  (params (OverlappedComponent :type "PrimitiveComponent Object Reference") (OtherActor :type "Actor Object Reference") (OtherComp :type "PrimitiveComponent Object Reference") (OtherBodyIndex :type Integer) (bFromSweep :type Boolean) (SweepResult :type "HitResult Structure (by ref)"))
  (bind _asbp_master_character (cast `/Game/RootMotionController/Blueprints/Character/BP_MasterCharacter` OtherActor))
  (if (`self.SmallNotification?`)
    (bind _root_motion_controller (`/Game/RootMotionController/Blueprints/Character/BP_MasterCharacter.Root Motion Controller` _asbp_master_character))
    (`/Game/RootMotionController/Blueprints/Components/BP_RootMotionController.Display Notification` _root_motion_controller (`self.DisplayTime`) (`self.Text`) (`self.TextColor`) (`self.UseMaterialInstance`) (`self.Icon`) (`self.IconAsTexture2D`) (`self.Texture2DTint`))
    (`self.K2_DestroyActor`)
    (else
      (`/Game/RootMotionController/Blueprints/Components/BP_RootMotionController.Display Big Notification` _root_motion_controller (`self.Headline`) (`self.HeadlineColor`) (`self.Description`) (`self.DescriptionColor`) (`self.Texture`) (`self.ImageFrameColor`))
      (`self.K2_DestroyActor`))))

(fn `UserConstructionScript`
  (bind (_triggerboxextent_x _triggerboxextent_y _triggerboxextent_z) (`KismetMathLibrary.BreakVector` (`self.TriggerBoxExtent`)))
  (bind _box (`self.Box`))
  (bind (_triggerboxextent_x_2 _triggerboxextent_y_2 _triggerboxextent_z_2) (`KismetMathLibrary.BreakVector` (`self.TriggerBoxExtent`)))
  (bind (_returnvalue_x _returnvalue_y) (`KismetMathLibrary.BreakVector` (`SceneComponent.K2_GetComponentLocation` _box)))
  (bind (_returnvalue_x_2 _returnvalue_y_2 _returnvalue_z) (`KismetMathLibrary.BreakVector` (`SceneComponent.K2_GetComponentLocation` (`self.Billboard`))))
  (`BoxComponent.SetBoxExtent` _box (`KismetMathLibrary.MakeVector` _triggerboxextent_x _triggerboxextent_y _triggerboxextent_z) true)
  (`SceneComponent.K2_SetWorldLocation` _box (`KismetMathLibrary.MakeVector` _returnvalue_x _returnvalue_y (+ _returnvalue_z _triggerboxextent_z_2)) false false)
  (`TextRenderComponent.K2_SetText` (`self.TextRender`) (`self.Text`)))