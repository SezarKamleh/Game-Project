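; BP_MasterCharacter_Child is a child character Blueprint that hooks the inherited player character up to a RootMotionController.
; On BeginPlay it passes itself, its pistol, rifle, sword and shield references, both cameras and the camera boom to the controller.
; Each Tick it feeds the magnitude of the movement component's last input vector as forward input, with directional forward input fixed at zero.
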(event `self.ReceiveBeginPlay`
  (`parent.ReceiveBeginPlay`)
  (message `/Game/RootMotionController/Blueprints/Interfaces/BPI_RMControllerInterface.InitializePlayer` (`self.Root Motion Controller`) self (`self.Pistol`) (`self.Rifle`) (`self.Sword`) (`self.Shield`) (`self.FollowCamera`) (`self.FPCamera`) (`self.CameraBoom`)))

(event `self.ReceiveTick`
  (params (DeltaSeconds :type "Float (single-precision)"))
  (`parent.ReceiveTick` DeltaSeconds)
  (`/Game/RootMotionController/Blueprints/Components/BP_RootMotionController.MoveForwardInput` (`self.Root Motion Controller`) (`KismetMathLibrary.VSize` (`PawnMovementComponent.GetLastInputVector` (`self.CharacterMovement`))) 0.0))

(fn `UserConstructionScript`
  (`parent.UserConstructionScript`))