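; Master AI pawn that drives a character through the RootMotionController component.
; BeginPlay initializes the controller as if for a player, passing itself, weapon references, cameras and the camera boom.
; Each Tick turns the length of CharacterMovement's last input vector into forward input, so AI movement requests feed the controller.
; Strafe input is an unwired placeholder, and a small DemoBranch macro gates on DemoCanMove.
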(event `self.ReceiveBeginPlay`
  ;[1 0.4794 0 1 16] Initialize Player
  (`/Game/RootMotionController/Blueprints/Interfaces/BPI_RMControllerInterface.InitializePlayer` (`self.Root Motion Controller`) self (`self.Pistol`) (`self.Rifle`) (`self.Sword`) (`self.Shield`) (`self.FollowCamera`) (`self.FPCamera`) (`self.CameraBoom`)))

(event `self.ReceiveTick`
  (params (DeltaSeconds :type "Float (single-precision)"))
  ;[0 0 0 1 16] Add Move Forward Input When AI Wants to Move
  (`/Game/RootMotionController/Blueprints/Components/BP_RootMotionController.MoveForwardInput` (`self.Root Motion Controller`) (`KismetMathLibrary.VSize` (`PawnMovementComponent.GetLastInputVector` (`self.CharacterMovement`))) 0.0))

(fn `UserConstructionScript`)