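; Master weapon Blueprint that assembles a weapon's visuals and applies camera recoil to a character.
; The construction script uses WeaponSettings to set the skeletal mesh, the sight mesh and its position, and the ironsight camera position.
; Separate yaw and pitch recoil events restart timelines that, on each update, feed a scaled-down, negated random value from the given range into the character's controller input.
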(event `Add Yaw Input For Recoil`
  (params (Character :type "Actor Object Reference") (`Yaw Min` :type "Float (double-precision)") (`Yaw Max` :type "Float (double-precision)"))
  (bind _ascharacter (cast `Character` Character))
  (`Timeline|Recoil Yaw` :!via `PlayFromStart`
    (:`Update`
      (`Pawn.AddControllerYawInput` _ascharacter (* (/ (`KismetMathLibrary.RandomFloatInRange` `Yaw Min` `Yaw Max`) 10.0) -1.0)))))

(event `Add Pitch Input For Recoil`
  (params (Character :type "Actor Object Reference") (PitchMin :type "Float (double-precision)") (PitchMax :type "Float (double-precision)"))
  (bind _ascharacter (cast `Character` Character))
  (`Timeline|Recoil Pitch` :!via `PlayFromStart`
    (:`Update`
      (`Pawn.AddControllerPitchInput` _ascharacter (* (/ (`KismetMathLibrary.RandomFloatInRange` PitchMin PitchMax) 10.0) -1.0)))))

(fn `UserConstructionScript`
  (bind (_weaponsettings_skeletalmesh _weaponsettings_sightmesh _weaponsettings_sightmeshlocation _weaponsettings_ironsightcameralocation) (break `/Game/RootMotionController/Blueprints/Weapon/BPS_WeaponSettings` (`self.WeaponSettings`)))
  (`SkinnedMeshComponent.SetSkinnedAssetAndUpdate` (`self.SkeletalMesh`) _weaponsettings_skeletalmesh true)
  (`StaticMeshComponent.SetStaticMesh` (`self.Sight`) _weaponsettings_sightmesh)
  (`SceneComponent.K2_SetRelativeLocation` (`self.Sight`) _weaponsettings_sightmeshlocation false false)
  (`SceneComponent.K2_SetRelativeLocation` (`self.Camera`) _weaponsettings_ironsightcameralocation false false))