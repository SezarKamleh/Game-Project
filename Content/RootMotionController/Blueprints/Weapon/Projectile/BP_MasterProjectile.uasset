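; BP_MasterProjectile is a projectile Blueprint in the RootMotionController weapon folder that handles impact feedback when it hits something.
; On Hit, it spawns a particle and plays a sound at the impact point, choosing character or wall variants by casting the hit actor to Character.
; It also places a short-lived impact decal oriented along the inverted hit normal, then destroys itself.
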(event `self.ReceiveHit`
  (params (MyComp :type "PrimitiveComponent Object Reference") (Other :type "Actor Object Reference") (OtherComp :type "PrimitiveComponent Object Reference") (bSelfMoved :type Boolean) (HitLocation :type "Vector Structure") (HitNormal :type "Vector Structure") (NormalImpulse :type "Vector Structure") (Hit :type "HitResult Structure (by ref)"))
  (bind (_ascharacter _bsuccess) (cast `Character` Other :!pure true))
  (bind _returnvalue (`KismetMathLibrary.Conv_VectorToRotator` (* HitNormal -1.0)))
  (`GameplayStatics.SpawnEmitterAtLocation` (select `bool` _bsuccess :`false` (`self.WallImpactParticle`) :`true` (`self.CharacterImpactParticle`)) HitLocation _returnvalue)
  (`GameplayStatics.SpawnDecalAtLocation` (`self.ImpactDecal`) (`self.DecalSize`) HitLocation _returnvalue 3.0)
  (`GameplayStatics.PlaySoundAtLocation` (select `bool` _bsuccess :`false` (`self.WallImpactSound`) :`true` (`self.CharacterImpactSound`)) HitLocation)
  (`self.K2_DestroyActor`))

(fn `UserConstructionScript`)